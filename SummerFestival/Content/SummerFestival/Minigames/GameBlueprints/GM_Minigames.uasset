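; Game mode for Summer Festival minigames that runs a match countdown and starts the objective targets.
; StartMatchTimer sets the game state's TotalSeconds from Minutes and starts a looping one-second timer.
; It then shows the timer widget and activates movement on every BP_Objective in the level.
; Each tick decrements TotalSeconds and clears the timer when it reaches zero.
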(event `StartMatchTimer`
  (bind _asgs_minigames (cast `/Game/SummerFestival/Minigames/GameBlueprints/GS_Minigames` (`GameplayStatics.GetGameState`)))
  (set `/Game/SummerFestival/Minigames/GameBlueprints/GS_Minigames.TotalSeconds` (`self.Minutes`) _asgs_minigames)
  (bind _returnvalue (`KismetSystemLibrary.K2_SetTimerDelegate` (delegate `TickTimer`) 1.0 true))
  (set `self.TimeHandler` _returnvalue)
  (`self.ShowUIandStartTargets`))

(event `TickTimer`
  (bind _output_get (set `/Game/SummerFestival/Minigames/GameBlueprints/GS_Minigames.TotalSeconds` (- (`/Game/SummerFestival/Minigames/GameBlueprints/GS_Minigames.TotalSeconds` (stale `StartMatchTimer` _asgs_minigames)) 1) (stale `StartMatchTimer` _asgs_minigames)))
  (if (<= _output_get 0)
    (`KismetSystemLibrary.K2_ClearAndInvalidateTimerHandle` (`self.TimeHandler`))))

(event `ShowUIandStartTargets`
  (bind _returnvalue (`|CreateWidget` "/Game/SummerFestival/UI/Widgets/WBP_Timer.WBP_Timer_C"))
  (`UserWidget.AddToViewport` _returnvalue 0)
  (bind _outactors (`GameplayStatics.GetAllActorsOfClass` "/Game/SummerFestival/Minigames/Blueprints/BP_Objective.BP_Objective_C"))
  (for _array_element _outactors
    (`/Game/SummerFestival/Minigames/Blueprints/BP_Objective.ActiveMovement` _array_element)))

(fn `UserConstructionScript`)