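; Player controller for the Summer Festival minigames, managing the local player's HUD and winner screen.
; On BeginPlay, the local controller adds the timer widget, switches to game-only input and hides the cursor.
; ActiveLocalCamera activates FPS mode on every BP_Minigame for player character 0 and calls its server start-movement event.
; ShowWinner swaps the timer for a winner screen with name and icon, using UI-only input.
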(event `self.ReceiveBeginPlay`
  (if (`self.IsLocalPlayerController`)
    (bind _returnvalue (`|CreateWidget` "/Game/SummerFestival/UI/Widgets/WBP_Timer.WBP_Timer_C" self))
    (set `self.TimerPointsWidget` _returnvalue)
    (`UserWidget.AddToViewport` _returnvalue 0)
    (`WidgetBlueprintLibrary.SetInputMode_GameOnly` self)
    (set `self.bShowMouseCursor` false)))

(event `ActiveLocalCamera`
  (bind _outactors (`GameplayStatics.GetAllActorsOfClass` "/Game/SummerFestival/Minigames/Blueprints/BP_Minigame.BP_Minigame_C"))
  (for _array_element _outactors
    (`/Game/SummerFestival/Minigames/Blueprints/BP_Minigame.ActiveFPSMinigame` _array_element (`GameplayStatics.GetPlayerCharacter` 0))
    (`/Game/SummerFestival/Minigames/Blueprints/BP_Minigame.RCP_ServerStartMovement` _array_element)))

(event `ShowWinner`
  (params (WinnerName :type Text) (WinnerIcon :type Name))
  (`Widget.RemoveFromParent` (`self.TimerPointsWidget`))
  (`WidgetBlueprintLibrary.SetInputMode_UIOnlyEx` self null)
  (bind _returnvalue (`|CreateWidget` "/Game/SummerFestival/UI/Widgets/WBP_WinnerScreen.WBP_WinnerScreen_C" null WinnerName WinnerIcon))
  (`UserWidget.AddToViewport` _returnvalue 0))

(fn `UserConstructionScript`)