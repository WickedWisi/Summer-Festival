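; BP_Objective is a scoring target for a Summer Festival minigame, configured by a data table row.
; The row sets its mesh and material at construction, and its movement speed and point value at runtime.
; ActiveMovement plays a timeline that lerps the actor between two offsets from its start position.
; Impact awards the row's points to the instigator's PS_Minigames player state through RCPAddpoints.
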(event `self.ReceiveBeginPlay`
  (set `self.InicialPos` (`self.K2_GetActorLocation`))
  (bind _returnvalue (`|GetDataTableRow` (`self.DataTableRef`) (`self.RowName`))
    (:`then`
      (`TimelineComponent.SetPlayRate` (`self.Movement`) (`.Velocity_15_8529E0044C9BD200384C2D8ED99E20A4` (break `/Game/SummerFestival/Minigames/Struct/S_Objectives` _returnvalue))))))

(event `ActiveMovement`
  (bind (_direction _movement) (`Timeline|Movement`)
    (:`Update`
      (`self.K2_SetActorLocation` (`KismetMathLibrary.VLerp` (+ (`self.Point`) (`self.InicialPos`)) (+ (`self.InicialPos`) (`self.Point 2`)) _movement)))))

(event `Impact`
  (bind _asps_minigames (cast `/Game/SummerFestival/Minigames/GameBlueprints/PS_Minigames` (`Pawn.PlayerState` (`self.GetInstigator`))))
  (`/Game/SummerFestival/Minigames/GameBlueprints/PS_Minigames.RCP_Addpoints` _asps_minigames (`.Points_8_AFE275D4440F1233CE9409A47BC55929` (break `/Game/SummerFestival/Minigames/Struct/S_Objectives` (stale `self.ReceiveBeginPlay` _returnvalue)))))

(fn `UserConstructionScript`
  (bind _objective (`self.Objective`))
  (bind _returnvalue (`|GetDataTableRow` (`self.DataTableRef`) (`self.RowName`))
    (:`then`
      (bind (_id _staticmesh _points _material) (break `/Game/SummerFestival/Minigames/Struct/S_Objectives` _returnvalue))
      (`StaticMeshComponent.SetStaticMesh` _objective _staticmesh)
      (`PrimitiveComponent.SetMaterial` _objective 0 _material))))