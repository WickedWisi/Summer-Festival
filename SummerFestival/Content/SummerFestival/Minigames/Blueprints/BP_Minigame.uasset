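; BP_Minigame runs a first-person shooting minigame with moving targets in the Summer Festival game.
; ActiveFPSMinigame enables shooting on a BP_ThirdPersonCharacter, ignores its move input, and switches it to the minigame camera using the Arrow component's rotation.
; A server-named RCP event calls RCP_StartTargetsMovement, which finds every BP_Objective in the level and activates its movement.
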(event `ActiveFPSMinigame`
  (params (Character :type "Actor Object Reference"))
  (bind _asbp_third_person_character (cast `/Game/ThirdPerson/Blueprints/BP_ThirdPersonCharacter` Character))
  (set `/Game/ThirdPerson/Blueprints/BP_ThirdPersonCharacter.CanShoot` true _asbp_third_person_character)
  (`Controller.SetIgnoreMoveInput` (`Pawn.GetController` _asbp_third_person_character) true)
  (`/Game/ThirdPerson/Blueprints/BP_ThirdPersonCharacter.ActiveMinigameCamera` _asbp_third_person_character (`SceneComponent.K2_GetComponentRotation` (`self.Arrow`))))

(event `RCP_StartTargetsMovement`
  (bind _outactors (`GameplayStatics.GetAllActorsOfClass` "/Game/SummerFestival/Minigames/Blueprints/BP_Objective.BP_Objective_C"))
  (for _array_element _outactors
    (`/Game/SummerFestival/Minigames/Blueprints/BP_Objective.ActiveMovement` _array_element)))

(event `RCP_ServerStartMovement`
  (`self.RCP_StartTargetsMovement`))

(fn `UserConstructionScript`)