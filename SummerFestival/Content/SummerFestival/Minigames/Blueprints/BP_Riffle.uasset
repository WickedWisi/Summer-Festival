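; BP_Riffle is a rifle actor for a Summer Festival minigame that fires projectiles.
; Its RCP_Shoot event spawns a BP_Bullet at the Arrow component's world location and rotation, regardless of collisions.
; An unconnected hitscan path, which would trace from the owning character's FPS camera and call Impact on a hit BP_Objective, never runs.
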(event `RCP_Shoot`
  (bind _arrow (`self.Arrow`))
  (`|SpawnActorFromClass` "/Game/SummerFestival/Minigames/Blueprints/BP_Bullet.BP_Bullet_C" (`KismetMathLibrary.MakeTransform` (`SceneComponent.K2_GetComponentLocation` _arrow) (`SceneComponent.K2_GetComponentRotation` _arrow)) "AlwaysSpawn" "MultiplyWithRoot" null null))

(fn `UserConstructionScript`)